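; Player-controlled Marine pawn that moves along fixed world X/Y axes from input and turns to follow the direction of mouse movement.
; Each tick, mouse delta over frame time gives a velocity, and rotation updates only when its length exceeds a dead zone.
; Atan2 of that velocity sets the controller's yaw directly, with pitch and roll zeroed.
; An RInterpTo node for smoothing is present but unconnected.
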(event EventTick
  (params (DeltaSeconds :type Float%20%28single-precision%29))
  (CallFunction|UpdatePlayerRotation))

(event Input|AxisEvents|InputAxisMoveForwardBack
  (params (AxisValue :type Float%20%28single-precision%29))
  ;[1 0.08854 0.08854] movement
  (Pawn|Input|AddMovementInput "1.000000, 0, 0" AxisValue false))

(event Input|AxisEvents|InputAxisMoveleftright
  (params (AxisValue :type Float%20%28single-precision%29))
  ;[1 0.08854 0.08854] movement
  (Pawn|Input|AddMovementInput "0,1.000000, 0" AxisValue false))

(fn ConstructionScript)

(fn IsMouseAbovetheZone
  ;[1 0.269 0.8665] czy gracz zaczął ruszać myszą/przekroczenie jednostki
  (return (> (Math|Vector2D|Vector2DLength (CallFunction|MouseVelocity)) (Variables|Default|GetMouseDeadZone))))

(fn MouseVelocity
  (bind _returnvalue (Game|GetPlayerController 0))
  (bind (_deltax _deltay) (Class|PlayerController|GetInputMouseDelta _returnvalue))
  ;[0.4792 0.4792 0.4792] Prędkosc myszy
  ;[1 1 1] info zwrotne
  (return (/ (Math|Vector2D|MakeVector2D _deltax _deltay) (Utilities|Time|GetWorldDeltaSeconds))))

(fn UpdatePlayerRotation
  (bind _returnvalue (CallFunction|MouseVelocity))
  ;[1 1 1] obrot naszej postaci
  ;[0 0 0 1 15] martwa strefa funkcja
  (if (CallFunction|IsMouseAbovetheZone)
    (Pawn|SetControlRotation (Game|GetPlayerController 0) (Math|Rotator|MakeRotator 0.0 0.0 (Class|KismetMathLibrary|DegAtan2 (.x _returnvalue) (.y _returnvalue))))))